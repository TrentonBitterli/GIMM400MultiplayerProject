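; Climbable ladder interactable that lets a player character move up and down while inside its box.
; Interact, if the character overlaps the box, enables ladder input for that player's indexed controller and switches movement to Flying.
; IA_Move's Y value then drives the stored character along its up vector.
; Leaving the box disables that input and restores Walking.
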(event `/Game/BoomerShooter/CouchCoop/Interfaces/BPI_Interactable.Interact`
  (params (Character :type "/Game/BoomerShooter/CouchCoop/Blueprints/ThirdPersonCharacter Object Reference"))
  (bind _output_get (set `self.Character` Character))
  ;[1 1 1] Is player overlaping (near ladder)
  (if (`PrimitiveComponent.IsOverlappingActor` (`self.Box`) _output_get)
    (`self.EnableInput` (`GameplayStatics.GetPlayerControllerFromID` (`/Game/BoomerShooter/CouchCoop/Blueprints/ThirdPersonCharacter.Index` _output_get)))
    (`CharacterMovementComponent.SetMovementMode` (`Character.CharacterMovement` _output_get) "MOVE_Flying" 0)))

(event `EnhancedInput|/Game/BoomerShooter/CouchCoop/Input/Actions/IA_Move`
  (params (ActionValue :type "Vector2D Structure") (ElapsedSeconds :type "Float (double-precision)") (TriggeredSeconds :type "Float (double-precision)") (InputAction :type "InputAction Object Reference" :default "/Game/BoomerShooter/CouchCoop/Input/Actions/IA_Move.IA_Move"))
  (bind _character (`self.Character`))
  (:`Triggered`
    (`Pawn.AddMovementInput` _character (`self.GetActorUpVector` _character) ActionValue_Y false)))

(event `self.Box.OnComponentEndOverlap`
  (params (OverlappedComponent :type "PrimitiveComponent Object Reference") (OtherActor :type "Actor Object Reference") (OtherComp :type "PrimitiveComponent Object Reference") (OtherBodyIndex :type Integer))
  (bind _asthird_person_character (cast `/Game/BoomerShooter/CouchCoop/Blueprints/ThirdPersonCharacter` OtherActor))
  (`self.DisableInput` (`GameplayStatics.GetPlayerControllerFromID` (`/Game/BoomerShooter/CouchCoop/Blueprints/ThirdPersonCharacter.Index` _asthird_person_character)))
  (`CharacterMovementComponent.SetMovementMode` (`Character.CharacterMovement` _asthird_person_character) "MOVE_Walking" 0))

(fn `UserConstructionScript`
  (`parent.UserConstructionScript`))